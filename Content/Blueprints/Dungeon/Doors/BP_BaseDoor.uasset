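; Base dungeon door Blueprint that opens, closes and unlocks when interacted with.
; Interact toggles an unlocked door, or spends an end key from the caller's component to unlock RoomA and RoomB.
; A dot product sets the swing away from the caller, and Tick eases CurrentDoorAngle toward the target set by open/close events.
; Lock changes and BeginPlay call UpdateMaterial, a hook for child classes.
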(event `self.ReceiveBeginPlay`
  (`self.Update Material` :!label _label))

(event `Update Material`)

(event `self.OnDoorLock_BP`
  (goto _label))

(event `self.OnDoorUnlock_BP`
  (goto _label))

(event `self.ReceiveTick`
  (params (DeltaSeconds :type "Float (single-precision)"))
  (bind _output_get (set `self.CurrentDoorAngle` (`KismetMathLibrary.FInterpTo` (`self.CurrentDoorAngle`) (`self.TargetDoorAngle`) DeltaSeconds 3.0)))
  (if (`KismetMathLibrary.NearlyEqual_FloatFloat` _output_get (`self.TargetDoorAngle`) 0.1)
    (set `self.CurrentDoorAngle` (`self.TargetDoorAngle`))))

(event `/Game/Blueprints/Interfaces/IInteractable.Interact`
  (params (Caller :type "Actor Object Reference"))
  (bind _returnvalue (message `/Game/Blueprints/Interfaces/IInteractable.CanInteract` self Caller))
  (if _returnvalue
    (if (`self.IsLocked`)
      (`self.TryUnlockDoor` Caller)
      (else
        (`self.Open` (not (`self.IsOpen`)))
        (set `self.Direction` (`KismetMathLibrary.SignOfFloat` (`KismetMathLibrary.Dot_VectorVector` (- (`self.K2_GetActorLocation` Caller) (`self.K2_GetActorLocation`)) (`self.GetActorForwardVector`))))))))

(event `self.OnDoorOpen_BP`
  (set `self.TargetDoorAngle` (* -90.0 (`self.Direction`))))

(event `self.OnDoorClose_BP`
  (set `self.TargetDoorAngle` 0.0))

(fn `CanInteract`
  (params (Caller :type "Actor Object Reference"))
  (returns (ReturnValue :type Boolean))
  (return true))

(fn `TryUnlockDoor`
  (params (Caller :type "Actor Object Reference"))
  (bind _returnvalue (`self.GetComponentByClass` Caller null))
  (`/Engine/EditorBlueprintResources/StandardMacros.IsValid` _returnvalue
    (:`Is Valid`
      (if (`/Game/Blueprints/Dungeon/Doors/BP_BaseDoor.HasEndKey` _returnvalue)
        (`self.RemoveEndKey` _returnvalue)
        ;[1 1 1] Should be both valid with this door actor
        (`Room.Lock` (`self.RoomA`) false)
        (`Room.Lock` (`self.RoomB`) false)
        (else
          (`KismetSystemLibrary.PrintString` "UNLOCK: No key" true true (struct :`R` 1.0 :`G` 0.087707 :`A` 1.0) 5.0))))
    (:`Is Not Valid`
      (`KismetSystemLibrary.PrintString` "UNLOCK: No Inventory Component" true true (struct :`R` 1.0 :`G` 0.087707 :`A` 1.0) 5.0))))

(fn `UserConstructionScript`)