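; Dungeon generator Blueprint that sets the starting room and respawns the player once a layout has been generated.
; ChooseFirstRoom always returns the StartRoom variable, and the pre- and post-generation events call their parent implementations.
; After generation, a non-empty room graph prints a success message and calls RestartPlayer on BP_MyPlayerController for player 0.
; An empty graph only prints a message that no rooms are available.
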(event `self.OnPreGeneration`
  (`parent.OnPreGeneration`))

(event `self.OnPostGeneration`
  (`parent.OnPostGeneration`)
  (if (> (`DungeonGraph.Count` (`self.Graph`)) 0)
    (`KismetSystemLibrary.PrintString` "Dungeon Generated")
    (bind _asbp_my_player_controller (cast `/Game/Blueprints/Player/BP_MyPlayerController` (`GameplayStatics.GetPlayerController` 0)))
    (`/Game/Blueprints/Player/BP_MyPlayerController.RestartPlayer` _asbp_my_player_controller)
    (else
      (`KismetSystemLibrary.PrintString` "No rooms available!"))))

(fn `Choose First Room`
  (returns (`Return room` :type "/Game/Blueprints/Dungeon/BP_MyRoom Object Reference"))
  (return (`self.Start room`)))

(fn `UserConstructionScript`)