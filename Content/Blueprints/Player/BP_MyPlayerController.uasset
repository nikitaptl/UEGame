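; BP_MyPlayerController is a player controller that lets input trigger procedural dungeon generation, unloading and respawning.
; The Generate and Unload input actions fire events that call Generate or Unload on the first DungeonGenerator actor found in the level.
; A RestartPlayer event respawns the player through the game mode at the player start named "Dungeon Start".
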(event `RestartPlayer`
  (bind _returnvalue (`GameplayStatics.GetGameMode`))
  ;[1 1 1] Teleport Player to Dungeon Start
  (`GameModeBase.RestartPlayerAtPlayerStart` _returnvalue self (`GameModeBase.K2_FindPlayerStart` _returnvalue self "Dungeon Start")))

(event `EnhancedInput|/Game/Input/Input_Generate`
  (params (ActionValue :type Boolean) (ElapsedSeconds :type "Float (double-precision)") (TriggeredSeconds :type "Float (double-precision)") (InputAction :type "InputAction Object Reference" :default "/Game/Input/Input_Generate.Input_Generate"))
  (:`Triggered`
    (`self.GenerateDungeon`)))

(event `GenerateDungeon`
  ;[1 1 1] Generate dungeon
  (bind _outactors (`GameplayStatics.GetAllActorsOfClass` "/Script/ProceduralDungeon.DungeonGenerator"))
  (`DungeonGeneratorBase.Generate` (`|GetArrayItem` _outactors)))

(event `EnhancedInput|/Game/Input/Input_Unload`
  (params (ActionValue :type Boolean) (ElapsedSeconds :type "Float (double-precision)") (TriggeredSeconds :type "Float (double-precision)") (InputAction :type "InputAction Object Reference" :default "/Game/Input/Input_Unload.Input_Unload"))
  (:`Triggered`
    (`self.UnloadDungeon`)))

(event `UnloadDungeon`
  ;[1 1 1] Unload dungeon
  (bind _outactors (`GameplayStatics.GetAllActorsOfClass` "/Script/ProceduralDungeon.DungeonGenerator"))
  (`DungeonGeneratorBase.Unload` (`|GetArrayItem` _outactors)))

(fn `UserConstructionScript`)